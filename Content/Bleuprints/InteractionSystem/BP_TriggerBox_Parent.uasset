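; Parent trigger box Blueprint for the interaction system that switches linked systems when the player character enters its Box component.
; Each begin overlap loops through SystemsToActivate, calls Activation or Deactivation based on each system's own Activated flag, then flips that flag.
; The trigger also flips its own Activated state, which blocks further toggling when ActivatableOnce is set.
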(event OnComponentBeginOverlap(Box)
  (params (OverlappedComponent :type Primitive%20Component%20Object%20Reference) (OtherActor :type Actor%20Object%20Reference) (OtherComp :type Primitive%20Component%20Object%20Reference) (OtherBodyIndex :type Integer) (bFromSweep :type Boolean) (SweepResult :type Hit%20Result%20Structure%20%28by%20ref%29))
  ;[0 1 0.9293] Detect player, then activate or deactivate all systems linked
  (if (== OtherActor (Game|GetPlayerCharacter 0))
    (if (not (and (Variables|Default|GetActivated?) (Variables|Default|GetActivatableOnce?)))
      (for _array_element (Variables|Default|GetSystemsToActivate)
        (if (Variables|/Game/Bleuprints/InteractionSystem/BP_System_Parent.BP_System_Parent_C|GetActivated%20? _array_element)
          (Default|Deactivation _array_element)
          (Variables|/Game/Bleuprints/InteractionSystem/BP_System_Parent.BP_System_Parent_C|SetActivated%20? _array_element false)
          (else
            (Default|Activation _array_element)
            (Variables|/Game/Bleuprints/InteractionSystem/BP_System_Parent.BP_System_Parent_C|SetActivated%20? _array_element true))))
      ;[0 1 0.9293] Set active true or false depending on current boolean value
      (if (Variables|Default|GetActivated?)
        (Variables|Default|SetActivated? false)
        (else
          (Variables|Default|SetActivated? true))))))

(event EventBeginPlay
  (|CallParentFunction) ; This node is disabled and will not be called.\nDrag off pins to build functionality.
)

(event Collision|EventActorBeginOverlap
  (params (OtherActor :type Actor%20Object%20Reference))
  (|CallParentFunction OtherActor) ; This node is disabled and will not be called.\nDrag off pins to build functionality.
)

(event EventTick
  (params (DeltaSeconds :type Float%20%28single-precision%29))
  (|CallParentFunction DeltaSeconds) ; This node is disabled and will not be called.\nDrag off pins to build functionality.
)

(fn ConstructionScript
  (|CallParentFunction))