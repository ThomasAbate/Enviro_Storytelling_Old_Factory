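; BP_Door is an interactable door in the interaction/keys system that swings open when activated and can close again.
; It overrides the parent's ActivatedAdditives and DeactivateAdditives hooks to play or reverse a Rotation timeline, which sets the SMDoor mesh's relative yaw.
; Comments note that Have Condition requires another interaction Blueprint to unlock it through Interaction To Unlock, and closing requires Interactable Once to be false.
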(event Custom|DoorRotation
  ;[1 0.4518 0.04025] Rotation animation of the door
  ;;[0 0 0 1 15] MODIFY "Rotation Movement" IF YOU WANT TO CHANGE THE ANIMATION (speed, back and forth...) !!
  (bind _rotation_movement (Timeline|Rotation Play)
    (:Update
      (Transformation|SetRelativeRotation (Variables|Default|GetSM_Door) (Math|Rotator|MakeRotator 0.0 0.0 _rotation_movement) false false))))

(event Custom|DoorClose
  ;[1 0.4518 0.04025] Rotation animation of the door
  ;;[0 0 0 1 15] MODIFY "Rotation Movement" IF YOU WANT TO CHANGE THE ANIMATION (speed, back and forth...) !!
  (bind _rotation_movement (Timeline|Rotation Reverse)
    (:Update
      (Transformation|SetRelativeRotation (Variables|Default|GetSM_Door) (Math|Rotator|MakeRotator 0.0 0.0 _rotation_movement) false false))))

(fn ConstructionScript
  (|CallParentFunction))

(fn ActivatedAdditives
  ;[1 0.4518 0.04025 1 16] Calls the animation when interacted with.
  ;
  ; If "Have Condition" is true, will only work if a child BP from the folder "InteractionSystem" references this blueprint in the variable"Interaction To Unlock" !
  ;
  ; If "Have Condition" is false, the anim will trigger if the player interacts with it.
  (CallFunction|DoorRotation))

(fn DeactivateAdditives
  ;[1 0.4518 0.04025] Plays if the player interacts and the boolean "Interactable Once" is false
  (CallFunction|DoorClose))