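; BP_Door is a lockable door that swings open once, when interacted with after being unlocked.
; Unlock sets a flag that IsInteract checks before a DoOnce plays the OpenDoorAnim timeline.
; The timeline lerps from the mesh's current relative rotation toward DoorOpenRota, applying the result as world rotation.
; The construction script poses the mesh at the open rotation, and BeginPlay resets it to zero relative rotation.
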(event EventIsInteract
  (bind _staticmesh (Variables|Default|GetStaticMesh))
  (if (Variables|Default|GetIs%20UnLock%20?%20)
    (Utilities|FlowControl|DoOnce false
      (:Completed
        (bind _alapha (Timeline|Open%20Door%20Anim Play)
          (:Update
            (Transformation|SetWorldRotation _staticmesh (Math|Rotator|Lerp(Rotator) (Variables|/Script/Engine.SceneComponent|GetRelativeRotation _staticmesh) (Variables|Default|GetDoor%20Open%20Rota) _alapha) false false)))))))

(event EventBeginPlay
  (Transformation|SetRelativeRotation (Variables|Default|GetStaticMesh) "0, 0, 0" false false))

(event EventUnlock
  (Variables|Default|SetIs%20UnLock%20?%20 true))

(fn ConstructionScript
  (|CallParentFunction)
  (Transformation|SetRelativeRotation (Variables|Default|GetStaticMesh) (Variables|Default|GetDoor%20Open%20Rota) false false))