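; BP_Final_Door is a door that teleports the player to a Target actor's location and rotation when they overlap its Box after it is unlocked.
; The Unlock event sets the IsUnLock flag that gates the teleport.
; The construction script poses the door at DoorOpenRota, and BeginPlay resets it to zero rotation.
; IsInteract ends at a DoOnce with no action, and the timeline door swing and DestroyActor are disconnected.
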(event OnComponentBeginOverlap(Box)
  (params (OverlappedComponent :type Primitive%20Component%20Object%20Reference) (OtherActor :type Actor%20Object%20Reference) (OtherComp :type Primitive%20Component%20Object%20Reference) (OtherBodyIndex :type Integer) (bFromSweep :type Boolean) (SweepResult :type Hit%20Result%20Structure%20%28by%20ref%29))
  (bind _returnvalue (Game|GetPlayerCharacter 0))
  (bind _target (Variables|Default|GetTarget))
  (bind _returnvalue_2 (Transformation|GetActorTransform _target))
  (if (and (== OtherActor _returnvalue) (Variables|Default|GetIs%20UnLock%20?%20))
    (Transformation|Teleport _returnvalue (.location _returnvalue_2) (.rotation _returnvalue_2))))

(event EventBeginPlay
  (Transformation|SetRelativeRotation (Variables|Default|GetDoor) "0, 0, 0" false false))

(event EventIsInteract
  (if (Variables|Default|GetIs%20UnLock%20?%20)
    (Utilities|FlowControl|DoOnce false)))

(event EventUnlock
  (Variables|Default|SetIs%20UnLock%20?%20 true))

(fn ConstructionScript
  (|CallParentFunction)
  (Transformation|SetRelativeRotation (Variables|Default|GetDoor) (Variables|Default|GetDoor%20Open%20Rota) false false))