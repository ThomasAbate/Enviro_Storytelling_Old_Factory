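; BP_Planche is a plank object that acts as a one-way teleport for the player once it is unlocked.
; An Unlock event sets the IsUnLock flag.
; When player character 0 begins overlapping the Box while that flag is set, it teleports to the Arrow component's world location with its rotation reset to zero.
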(event OnComponentBeginOverlap(Box)
  (params (OverlappedComponent :type Primitive%20Component%20Object%20Reference) (OtherActor :type Actor%20Object%20Reference) (OtherComp :type Primitive%20Component%20Object%20Reference) (OtherBodyIndex :type Integer) (bFromSweep :type Boolean) (SweepResult :type Hit%20Result%20Structure%20%28by%20ref%29))
  (if (and (== OtherActor (Game|GetPlayerCharacter 0)) (Variables|Default|GetIs%20UnLock%20?%20))
    (Transformation|Teleport (Game|GetPlayerCharacter 0) (Transformation|GetWorldLocation (Variables|Default|GetArrow)) "0, 0, 0")))

(event EventBeginPlay)

(event EventUnlock
  (Variables|Default|SetIs%20UnLock%20?%20 true))

(fn ConstructionScript
  (|CallParentFunction))