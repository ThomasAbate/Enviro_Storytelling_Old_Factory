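; BP_Loocker1 is a lockable door object that teleports the player to a Target's location and rotation once it is unlocked and interacted with.
; An Unlock event sets the flag that IsInteract checks, and a DoOnce limits the teleport to a single use.
; The construction script poses the Door at its open rotation, and BeginPlay resets it to zero.
; The Timeline door swing and the DestroyActor call are unwired.
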(event EventBeginPlay
  (Transformation|SetRelativeRotation (Variables|Default|GetDoor) "0, 0, 0" false false))

(event EventIsInteract
  (bind _target (Variables|Default|GetTarget))
  (bind _returnvalue (Transformation|GetActorTransform _target))
  (if (Variables|Default|GetIs%20UnLock%20?%20)
    (Utilities|FlowControl|DoOnce false
      (:Completed
        (Transformation|Teleport (Game|GetPlayerCharacter 0) (.location _returnvalue) (.rotation _returnvalue))))))

(event EventUnlock
  (Variables|Default|SetIs%20UnLock%20?%20 true))

(fn ConstructionScript
  (|CallParentFunction)
  (Transformation|SetRelativeRotation (Variables|Default|GetDoor) (Variables|Default|GetDoor%20Open%20Rota) false false))