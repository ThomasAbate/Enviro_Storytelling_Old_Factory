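; Blueprint actor that moves a mesh along a spline generated by a Houdini Digital Asset curve, looping continuously.
; On BeginPlay it casts the first child of the referenced HDA's Houdini asset component to a spline component and caches it.
; Each tick it sets the mesh's world location and rotation from the spline, using real time times a speed multiplier, wrapped by spline length, as distance.
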(event EventBeginPlay
  (bind _asspline_component (Utilities|Casting|CastToSplineComponent (Utilities|Array|Get(acopy) (Components|GetChildrenComponents (Variables|/Script/HoudiniEngineRuntime.HoudiniAssetActor|GetHoudiniAssetComponent (Variables|Default|GetHoudini_HDA_Curve)) false))))
  (Variables|Default|SetAs%20Spline%20Component _asspline_component))

(event Collision|EventActorBeginOverlap
  (params (OtherActor :type Actor%20Object%20Reference)))

(event EventTick
  (params (DeltaSeconds :type Float%20%28single-precision%29))
  (bind _returnvalue (Utilities|Time|GetRealTimeSeconds))
  (bind _as_spline_component (Variables|Default|GetAs%20Spline%20Component))
  (bind _time_mult (Variables|Default|GetTime_mult))
  (bind _returnvalue_2 (Spline|GetSplineLength _as_spline_component))
  (bind _returnvalue_3 (* _returnvalue _time_mult))
  (bind _returnvalue_4 (Math|Float|%(Float) _returnvalue_3 _returnvalue_2))
  (bind _returnvalue_5 (Spline|GetTransformatDistanceAlongSpline _as_spline_component _returnvalue_4 "World" false))
  (Transformation|SetWorldTransform (Variables|Default|GetMesh) (Math|Transform|MakeTransform (.location _returnvalue_5) (.rotation _returnvalue_5) "1.000000,1.000000,1.000000") false false))

(fn ConstructionScript)