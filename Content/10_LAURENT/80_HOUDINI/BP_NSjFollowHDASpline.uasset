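; BP_NSjFollowHDASpline moves a Niagara effect along a curve generated by a Houdini Digital Asset.
; On BeginPlay it takes the first child of the Houdini asset component and caches it as a spline component.
; Each tick it scales real time by a multiplier, wraps it by spline length, and moves the Niagara to that world location, looping along the curve.
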(event EventBeginPlay
  (bind _asspline_component (Utilities|Casting|CastToSplineComponent (Utilities|Array|Get(acopy) (Components|GetChildrenComponents (Variables|/Script/HoudiniEngineRuntime.HoudiniAssetActor|GetHoudiniAssetComponent (Variables|Default|GetHoudini_HDA_Curve)) false))))
  (Variables|Default|SetAs%20Spline%20Component _asspline_component))

(event Collision|EventActorBeginOverlap
  (params (OtherActor :type Actor%20Object%20Reference)))

(event EventTick
  (params (DeltaSeconds :type Float%20%28single-precision%29))
  (bind _as_spline_component (Variables|Default|GetAs%20Spline%20Component))
  (Transformation|SetWorldTransform (Variables|Default|GetNiagara) (Math|Transform|MakeTransform (.location (Spline|GetTransformatDistanceAlongSpline _as_spline_component (Math|Float|%(Float) (* (Utilities|Time|GetRealTimeSeconds) (Variables|Default|GetTime_mult)) (Spline|GetSplineLength _as_spline_component)) "World" false)) "0, 0, 0" "1.000000,1.000000,1.000000") false false))

(fn ConstructionScript)