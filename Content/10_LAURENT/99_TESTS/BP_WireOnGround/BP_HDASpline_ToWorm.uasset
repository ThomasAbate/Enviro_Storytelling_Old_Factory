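; Generated dynamic mesh test Blueprint that builds a cable lying on the ground from a curve of a Houdini HDA.
; On mesh rebuild, it picks the HDA's child spline by index, resamples it and line-traces each sample downward, dropping misses.
; The hits form a new spline component, which is resampled and swept with a circle profile via Geometry Script into an uncapped tube with adjustable radius, scale and rotation.
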(event Events|EventOnRebuildGeneratedMesh
  (params (TargetMesh :type Dynamic%20Mesh%20Object%20Reference))
  (Variables|Default|SetMyDynamicMesh TargetMesh)
  (Utilities|FlowControl|Sequence
    (:then_0
      (bind _asspline_component (Utilities|Casting|CastToSplineComponent (Utilities|Array|Get(acopy) (Components|GetChildrenComponents (Variables|/Script/Engine.Actor|GetRootComponent (Variables|CurveHDA|GetHoudiniHDA)) false) (Variables|CurveHDA|GetCurveNum))))
      (Variables|Default|SetAs%20Spline%20Component _asspline_component))
    (:then_1
      ;[0.4225 1 0.5105] Resample
      (bind _frames (Class|GeometryScriptLibraryPolyPathFunctions|SampleSplinetoTransforms :Spline (Variables|Default|GetAs%20Spline%20Component) :SamplingOptions (Utilities|Struct|MakeGeometryScriptSplineSamplingOptions (Variables|Default|GetPoint%20Sample) 1.0)))
      (Variables|Default|SetSplineResampledOriginal1 _frames))
    (:then_2
      (Utilities|Array|Clear (Variables|Default|GetSplinePointsProjected1)))
    (:then_3
      ;[0.3434 0.4724 1] Proj points to nearest surface
      (for _array_element (Variables|Default|GetSplineResampledOriginal1)
        (bind _outhit (Collision|LineTraceByChannel (Math|Transform|TransformLocation (Transformation|GetWorldTransform (Variables|Default|GetAs%20Spline%20Component)) (.Location (Math|Transform|BreakTransform _array_element))) (+ (Math|Transform|TransformLocation (Transformation|GetWorldTransform (Variables|Default|GetAs%20Spline%20Component)) (.Location (Math|Transform|BreakTransform _array_element))) (Math|Vector|MakeVector 0.0 0.0 (* (Variables|Default|GetLineTraceLength) -1.0))) "TraceTypeQuery1" true 0 "ForDuration" true "(R=1.000000,G=0.000000,B=0.000000,A=1.000000)" "(R=0.000000,G=1.000000,B=0.000000,A=1.000000)" 0.1))
        (if (.bBlockingHit (Collision|BreakHitResult _outhit))
          (Utilities|Array|Add (Variables|Default|GetSplinePointsProjected1) (Math|Transform|MakeTransform (Math|Transform|InverseTransformLocation (Transformation|GetWorldTransform (Variables|Default|GetAs%20Spline%20Component)) (.Location (Collision|BreakHitResult _outhit))) (.Rotation (Math|Transform|BreakTransform _array_element)) (.Scale (Math|Transform|BreakTransform _array_element)))))))
    (:then_4)
    (:then_5
      ;[0.702 1 0.3642] Make New Spline On Projected Points
      (bind _returnvalue (AddComponent|AddSplineComponent false))
      (bind _output_get (Variables|Default|SetSplineReprojected _returnvalue))
      (Spline|ClearSplinePoints _output_get true)
      (for (_array_element_2 _array_index) (Variables|Default|GetSplinePointsProjected1)
        (Spline|AddSplinePointatIndex _output_get (.location _array_element_2) _array_index "Local" false))
      (Spline|SetClosedLoop _output_get false false)
      (Spline|UpdateSpline _output_get))
    (:then_6
      ;[0.2575 0.3087 1] Generate The Cable Mesh
      (bind _frames_2 (Class|GeometryScriptLibraryPolyPathFunctions|SampleSplinetoTransforms :Spline (Variables|Default|GetSplineReprojected) :SamplingOptions (Utilities|Struct|MakeGeometryScriptSplineSamplingOptions (Variables|Default|GetPoint%20Sample) 1.0 "UniformDistance" "Local" "FullSpline" 0.0 1.0)))
      (bind _returnvalue_2 (Class|GeometryScriptLibraryPolyPathFunctions|CreateCirclePath3D :Radius (Variables|Default|GetCable%20Radius) :NumPoints (Variables|Default|GetColumns)))
      (Class|GeometryScriptLibraryMeshPrimitiveFunctions|AppendSweepPolygon (Variables|Default|GetMyDynamicMesh) (Utilities|Struct|MakeGeometryScriptPrimitiveOptions "PerFace" false "ScaleToFill") (Math|Transform|MakeTransform (Math|Vector|MakeVector 0.0 0.0 (/ (Variables|Default|GetCable%20Radius) 2.0))) (Class|GeometryScriptLibraryPolyPathFunctions|ToArrayOfVector2D(GeometryScriptPolyPath) _returnvalue_2) _frames_2 false false (Variables|Default|GetStart%20Scale) (Variables|Default|GetEnd%20Scale) (Variables|Default|GetRotation%20Angle%20Deg) 0))))

(fn ConstructionScript)