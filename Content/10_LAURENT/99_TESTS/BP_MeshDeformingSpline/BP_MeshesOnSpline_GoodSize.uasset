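; Test Blueprint that tiles a chosen static mesh along a spline at roughly its natural length, deforming each copy to the curve.
; The construction script derives the mesh's X length from its bounding box and divides the spline length by it to set the segment count.
; Each segment is an X-forward spline mesh component placed by distance along the spline, with tangents clamped to that length.
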(event EventBeginPlay)

(event Collision|EventActorBeginOverlap
  (params (OtherActor :type Actor%20Object%20Reference)))

(event EventTick
  (params (DeltaSeconds :type Float%20%28single-precision%29)))

(fn ConstructionScript
  (bind _meshinput (Variables|Default|GetMeshInput))
  (bind _spline (Variables|Default|GetSpline))
  (bind _spline_2 (Variables|Default|GetSpline))
  (bind _returnvalue (StaticMesh|GetBoundingBox _meshinput))
  (bind _output_get (Variables|Default|SetX_Length (.x (+ (Math|Vector|VectorGetAbs (.min _returnvalue)) (Math|Vector|VectorGetAbs (.max _returnvalue))))))
  (for _index (range 0 (Math|Float|Truncate (/ (Spline|GetSplineLength (Variables|Default|GetSpline)) _output_get)))
    (bind _returnvalue_2 (AddComponent|AddSplineMeshComponent false))
    (SplineMesh|SetForwardAxis _returnvalue_2 "X" true)
    (Components|StaticMesh|SetStaticMesh _returnvalue_2 (Variables|Default|GetMeshInput))
    (SplineMesh|SetStartandEnd _returnvalue_2 (Spline|GetLocationatDistanceAlongSpline _spline_2 (* _index (Variables|Default|GetX_Length)) "Local") (Math|Vector|ClampVectorSize (Spline|GetTangentatDistanceAlongSpline _spline_2 (* _index (Variables|Default|GetX_Length)) "Local") 0.0 (Variables|Default|GetX_Length)) (Spline|GetLocationatDistanceAlongSpline _spline (* (+ _index 1) (Variables|Default|GetX_Length)) "Local") (Math|Vector|ClampVectorSize (Spline|GetTangentatDistanceAlongSpline _spline (* (+ _index 1) (Variables|Default|GetX_Length)) "Local") 0.0 (Variables|Default|GetX_Length)) true :!class /Script/Engine.SplineMeshComponent)))