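; BP_ViewObject is an interaction-system object that toggles a view mode for the player.
; Both its activate and deactivate additive functions call ViewEvent, which flips an IsPaused flag.
; Entering shows the mouse cursor, ignores move and look input, and adds a W_Blur widget to the viewport.
; Exiting reverses this and removes the widget, without actually pausing the game.
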(event Custom|View%20Event
  (bind _returnvalue (Game|GetPlayerController 0))
  (if (Variables|Default|GetIs%20Paused)
    (Variables|/Script/Engine.PlayerController|SetbShowMouseCursor _returnvalue false)
    (Input|SetIgnoreMoveInput _returnvalue false)
    (Input|SetIgnoreLookInput _returnvalue false)
    (Variables|Default|SetIs%20Paused false)
    (Widget|RemovefromParent (stale _returnvalue_2))
    (else
      (Variables|/Script/Engine.PlayerController|SetbShowMouseCursor _returnvalue true)
      (Input|SetIgnoreMoveInput _returnvalue true)
      (Input|SetIgnoreLookInput _returnvalue true)
      (Variables|Default|SetIs%20Paused true)
      (bind _returnvalue_2 (UserInterface|CreateWidget "/Game/SystemsAndBlueprints/InteractionSystem/ViewObject/W_Blur.W_Blur_C"))
      (UserInterface|Viewport|AddtoViewport _returnvalue_2 0))))

(event EventBeginPlay
  (|CallParentFunction) ; This node is disabled and will not be called.\nDrag off pins to build functionality.
)

(event Collision|EventActorBeginOverlap
  (params (OtherActor :type Actor%20Object%20Reference)))

(event EventTick
  (params (DeltaSeconds :type Float%20%28single-precision%29)))

(fn ConstructionScript
  (|CallParentFunction))

(fn ActivatedAdditives
  (CallFunction|ViewEvent))

(fn DeactivateAdditives
  (CallFunction|ViewEvent))