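; BP_InspectItem is an interactable item in the interaction system's ViewObject feature, displaying a configurable mesh that is applied in the construction script.
; InteractItem returns that model to the caller and branches on the TakeObject flag.
; Takeable items destroy themselves after a short delay.
; Otherwise it triggers the don't-take event, where a FlipFlop alternately hides and shows the mesh in the world.
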(event Custom|Destroy
  (Utilities|FlowControl|Delay 0.2)
  (Actor|DestroyActor))

(event Custom|Event%20Dont%20Take
  (bind _staticmesh_0 (Variables|Default|GetStaticMesh_0))
  (Utilities|FlowControl|FlipFlop
    (:A
      (Rendering|SetVisibility _staticmesh_0 false false))
    (:B
      (Rendering|SetVisibility _staticmesh_0 true false))))

(fn ConstructionScript
  (Components|StaticMesh|SetStaticMesh (Variables|Default|GetStaticMesh_0) (Variables|Default|GetItemModel)))

(fn InteractItem
  (if (Variables|Default|GetTake%20Object)
    (CallFunction|Destroy)
    (else
      (CallFunction|EventDontTake)))
  (return (Variables|Default|GetItemModel)))