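; Room transition trigger in the interaction system that teleports the player to another spot once unlocked.
; An Activation function sets the Key flag, and nothing in this Blueprint clears it.
; When the player character overlaps the Box while Key is set, it teleports to the Target actor's location and rotation.
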(event OnComponentBeginOverlap(Box)
  (params (OverlappedComponent :type Primitive%20Component%20Object%20Reference) (OtherActor :type Actor%20Object%20Reference) (OtherComp :type Primitive%20Component%20Object%20Reference) (OtherBodyIndex :type Integer) (bFromSweep :type Boolean) (SweepResult :type Hit%20Result%20Structure%20%28by%20ref%29))
  (bind _target (Variables|Default|GetTarget))
  (bind _returnvalue (Transformation|GetActorTransform _target))
  (if (and (== OtherActor (Game|GetPlayerCharacter 0)) (Variables|Default|GetKey))
    (Transformation|Teleport (Game|GetPlayerCharacter 0) (.location _returnvalue) (.rotation _returnvalue))))

(fn ConstructionScript
  (|CallParentFunction))

(fn Activation
  (Variables|Default|SetKey true))