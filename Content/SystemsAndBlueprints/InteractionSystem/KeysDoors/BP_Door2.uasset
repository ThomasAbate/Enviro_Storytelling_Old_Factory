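; BP_Door2 is a sliding door in the interaction system that responds to additive activation and deactivation.
; Activation plays a timeline whose RotationMovement track, despite its name, lerps the mesh's relative location toward Destination.
; Deactivation reverses the timeline, but each update lerps from the current location rather than a stored start, so nothing moves the mesh back to its original position.
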(event Custom|DoorOpen
  (bind _staticmesh (Variables|Default|GetStaticMesh))
  ;[0 0 0 1 15] MODIFY "Rotation Movement" IF YOU WANT TO CHANGE THE ANIMATION (speed, back and forth...) !!
  (bind _rotation_movement (Timeline|Timeline Play)
    (:Update
      (Transformation|SetRelativeLocation _staticmesh (Math|Vector|Lerp(Vector) (Variables|/Script/Engine.SceneComponent|GetRelativeLocation _staticmesh) (Variables|Default|GetDestination) _rotation_movement) false false))))

(event Custom|DoorClosing
  (bind _staticmesh (Variables|Default|GetStaticMesh))
  ;[0 0 0 1 15] MODIFY "Rotation Movement" IF YOU WANT TO CHANGE THE ANIMATION (speed, back and forth...) !!
  (bind _rotation_movement (Timeline|Timeline Reverse)
    (:Update
      (Transformation|SetRelativeLocation _staticmesh (Math|Vector|Lerp(Vector) (Variables|/Script/Engine.SceneComponent|GetRelativeLocation _staticmesh) (Variables|Default|GetDestination) _rotation_movement) false false))))

(event EventBeginPlay
  (|CallParentFunction) ; This node is disabled and will not be called.\nDrag off pins to build functionality.
)

(event Collision|EventActorBeginOverlap
  (params (OtherActor :type Actor%20Object%20Reference)))

(event EventTick
  (params (DeltaSeconds :type Float%20%28single-precision%29)))

(fn ConstructionScript
  (|CallParentFunction))

(fn ActivatedAdditives
  (CallFunction|DoorOpen))

(fn DeactivateAdditives
  (CallFunction|DoorClosing))