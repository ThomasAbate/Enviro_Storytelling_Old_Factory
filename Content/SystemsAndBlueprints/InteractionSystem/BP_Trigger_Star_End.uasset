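; BP_Trigger_Star_End is a one-shot trigger that reveals a mesh with a sound cue when the player walks into it.
; On BeginPlay the static mesh is invisible and has no collision.
; The first Box overlap by the player character plays explosion and shocked 2D sounds, then makes the mesh visible with query and physics collision.
; A DoOnce prevents repeats.
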(event OnComponentBeginOverlap(Box)
  (params (OverlappedComponent :type Primitive%20Component%20Object%20Reference) (OtherActor :type Actor%20Object%20Reference) (OtherComp :type Primitive%20Component%20Object%20Reference) (OtherBodyIndex :type Integer) (bFromSweep :type Boolean) (SweepResult :type Hit%20Result%20Structure%20%28by%20ref%29))
  (bind _staticmesh (Variables|Default|GetStaticMesh))
  (if (== OtherActor (Game|GetPlayerCharacter 0))
    (Utilities|FlowControl|DoOnce false
      (:Completed
        (Audio|PlaySound2D "/Game/Sounds/SFX/Explosion.Explosion" 1.0 1.0 0.0 0 0)
        (Audio|PlaySound2D "/Game/Sounds/Voices/Shocked.Shocked" 1.0 1.0 0.0 0 0)
        (Rendering|SetVisibility _staticmesh true false)
        (Collision|SetCollisionEnabled _staticmesh "QueryAndPhysics")))))

(event EventBeginPlay
  (bind _staticmesh (Variables|Default|GetStaticMesh))
  (Rendering|SetVisibility _staticmesh false false)
  (Collision|SetCollisionEnabled _staticmesh "NoCollision"))

(fn ConstructionScript)