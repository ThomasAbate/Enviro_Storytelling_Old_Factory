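; Base Blueprint for pickable objects in the interaction system, which affects other interactions and systems when the player interacts with it.
; Interact sets ConditionTrue on each interaction in its unlock list, then toggles each linked system through Activation or Deactivation and flips its Activated flag.
; It finishes with a Niagara effect at the static mesh location and a 2D sound, without destroying or hiding itself here.
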(event EventBeginPlay
  (|CallParentFunction) ; This node is disabled and will not be called.\nDrag off pins to build functionality.
)

(event Collision|EventActorBeginOverlap
  (params (OtherActor :type Actor%20Object%20Reference)))

(event EventTick
  (params (DeltaSeconds :type Float%20%28single-precision%29)))

(event EventInteract
  (for _array_element (Variables|Default|GetInteractionsToUnlock_0)
    (Variables|/Game/SystemsAndBlueprints/InteractionSystem/BP_Interactable_Parent.BP_Interactable_Parent_C|SetConditionTrue? _array_element true))
  (for _array_element_2 (Variables|Default|GetSystemsToLink)
    (if (Variables|/Game/SystemsAndBlueprints/InteractionSystem/BP_System_Parent.BP_System_Parent_C|GetActivated%20? _array_element_2)
      (Default|Deactivation _array_element_2)
      (Variables|/Game/SystemsAndBlueprints/InteractionSystem/BP_System_Parent.BP_System_Parent_C|SetActivated%20? _array_element_2 false)
      (else
        (Default|Activation _array_element_2)
        (Variables|/Game/SystemsAndBlueprints/InteractionSystem/BP_System_Parent.BP_System_Parent_C|SetActivated%20? _array_element_2 true))))
  (Niagara|SpawnSystematLocation (Variables|Default|GetVFXPickableTaken) (Transformation|GetWorldLocation (Variables|Default|GetStaticMesh)))
  (Audio|PlaySound2D (Variables|Default|GetSoundActivated) 1.0 1.0 0.0 0 0))

(fn ConstructionScript
  (|CallParentFunction))